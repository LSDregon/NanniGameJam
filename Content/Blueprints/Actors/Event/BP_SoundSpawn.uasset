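; BP_SoundSpawn is an event actor that plays a 2D sound once when its EventListener reports the actor as enabled.
; Tick polls the listener, and the first time it is enabled, plays Sound and sets a flag that blocks replays.
; It then reports itself to the listener through TaskCompleted.
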(event EventBeginPlay)

(event Collision|EventActorBeginOverlap
  (params (OtherActor :type Actor%20Object%20Reference)))

(event EventTick
  (params (DeltaSeconds :type Float%20%28single-precision%29))
  (if (and (Class|EventListenerComponent|IsIsActorEnable (Variables|Default|GetEventListener)) (not (Variables|Default|GetAlready%20Activarted)))
    (Audio|PlaySound2D (Variables|Default|GetSound) 1.0 1.0 0.0 0 0)
    (Variables|Default|SetAlready%20Activarted true)
    (Class|EventListenerComponent|TaskCompleted (Variables|Default|GetEventListener) self)))

(fn ConstructionScript)