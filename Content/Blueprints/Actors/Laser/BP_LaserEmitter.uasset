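; BP_LaserEmitter is a laser emitter actor prototyping a beam that reflects off surfaces, currently drawn only as debug lines.
; Its TEST function loops line traces on TraceTypeQuery3, mirroring the direction at each impact normal until a trace misses, with no bounce cap.
; The delayed call that feeds TEST from LaserEmitterSource's location and forward vector is not wired to any event, so it never runs.
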(event EventBeginPlay)

(event Collision|EventActorBeginOverlap
  (params (OtherActor :type Actor%20Object%20Reference)))

(fn ConstructionScript)

(fn TEST
  (params (or :type Vector) (dir :type Vector) (dist :type Float%20%28double-precision%29))
  (Variables|Default|SetL_Or or)
  (Variables|Default|SetL_Dir dir)
  (Variables|Default|SetL_Dist dist)
  (while (Variables|Default|GetL_Continue)
    (bind (_outhit _returnvalue) (Collision|LineTraceByChannel (Variables|Default|GetL_Or) (+ (Variables|Default|GetL_Or) (* (Variables|Default|GetL_Dir) (Variables|Default|GetL_Dist))) "TraceTypeQuery3" true 0 "ForDuration" true "(R=1.000000,G=0.000000,B=0.000000,A=1.000000)" "(R=0.000000,G=1.000000,B=0.000000,A=1.000000)" 1e+01))
    (if _returnvalue
      (Variables|Default|SetL_Or (.ImpactPoint (Collision|BreakHitResult _outhit)))
      (Variables|Default|SetL_Dir (Math|Vector|MirrorVectorbyNormal (Variables|Default|GetL_Dir) (.ImpactNormal (Collision|BreakHitResult _outhit))))
      (else
        (Variables|Default|SetL_Continue false)))))