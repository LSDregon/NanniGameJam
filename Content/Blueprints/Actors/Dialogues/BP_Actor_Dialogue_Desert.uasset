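; Desert dialogue actor that plays a one-shot, five-line voice sequence with on-screen subtitles.
; Tick polls the EventListener and, unless it is in an event task with the actor disabled, latches IsActivated and reports the task completed.
; Timed delays step through five events, each pulling text and a 2D sound from the AudioText map.
; The player HUD's Summer overlay appears with the first line and hides after the last.
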(event Custom|Exec%20Sound%201
  (bind _audio_text (Variables|Default|GetAudio_Text))
  (bind _value (Utilities|Map|Find _audio_text 1))
  (bind (_sound _text) (Utilities|Struct|BreakStruct_Audio_Text _value))
  (bind _asbp_main_character (Utilities|Casting|CastToBP_MainCharacter (Game|GetPlayerCharacter 0)))
  (Default|SetTextSummer (Variables|/Game/Blueprints/MainPlayer/BP_MainCharacter.BP_MainCharacter_C|GetHUD _asbp_main_character) _text)
  (Widget|SetVisibility (Variables|/Game/Blueprints/MainPlayer/WBP_HUD.WBP_HUD_C|GetOverlay_Summer (Variables|/Game/Blueprints/MainPlayer/BP_MainCharacter.BP_MainCharacter_C|GetHUD _asbp_main_character)) "Visible")
  (Audio|PlaySound2D _sound 1.0 1.0 0.0 0 0))

(event Custom|Exec%20Sound%202
  (bind _audio_text (Variables|Default|GetAudio_Text))
  (bind _value (Utilities|Map|Find _audio_text 2))
  (bind (_sound _text) (Utilities|Struct|BreakStruct_Audio_Text _value))
  (bind _asbp_main_character (Utilities|Casting|CastToBP_MainCharacter (Game|GetPlayerCharacter 0)))
  (Default|SetTextSummer (Variables|/Game/Blueprints/MainPlayer/BP_MainCharacter.BP_MainCharacter_C|GetHUD _asbp_main_character) _text)
  (Audio|PlaySound2D _sound 1.0 1.0 0.0 0 0))

(event Custom|Exec%20Sound%203
  (bind _audio_text (Variables|Default|GetAudio_Text))
  (bind _value (Utilities|Map|Find _audio_text 3))
  (bind (_sound _text) (Utilities|Struct|BreakStruct_Audio_Text _value))
  (bind _asbp_main_character (Utilities|Casting|CastToBP_MainCharacter (Game|GetPlayerCharacter 0)))
  (Default|SetTextSummer (Variables|/Game/Blueprints/MainPlayer/BP_MainCharacter.BP_MainCharacter_C|GetHUD _asbp_main_character) _text)
  (Audio|PlaySound2D _sound 1.0 1.0 0.0 0 0))

(event Custom|Exec%20Sound%204
  (bind _audio_text (Variables|Default|GetAudio_Text))
  (bind _value (Utilities|Map|Find _audio_text 4))
  (bind (_sound _text) (Utilities|Struct|BreakStruct_Audio_Text _value))
  (bind _asbp_main_character (Utilities|Casting|CastToBP_MainCharacter (Game|GetPlayerCharacter 0)))
  (Default|SetTextSummer (Variables|/Game/Blueprints/MainPlayer/BP_MainCharacter.BP_MainCharacter_C|GetHUD _asbp_main_character) _text)
  (Audio|PlaySound2D _sound 1.0 1.0 0.0 0 0))

(event Custom|Exec%20Sound%205
  (bind _audio_text (Variables|Default|GetAudio_Text))
  (bind _value (Utilities|Map|Find _audio_text 5))
  (bind (_sound _text) (Utilities|Struct|BreakStruct_Audio_Text _value))
  (bind _asbp_main_character (Utilities|Casting|CastToBP_MainCharacter (Game|GetPlayerCharacter 0)))
  (Default|SetTextSummer (Variables|/Game/Blueprints/MainPlayer/BP_MainCharacter.BP_MainCharacter_C|GetHUD _asbp_main_character) _text)
  (Audio|PlaySound2D _sound 1.0 1.0 0.0 0 0)
  (Utilities|FlowControl|Delay 6.0)
  (Widget|SetVisibility (Variables|/Game/Blueprints/MainPlayer/WBP_HUD.WBP_HUD_C|GetOverlay_Summer (Variables|/Game/Blueprints/MainPlayer/BP_MainCharacter.BP_MainCharacter_C|GetHUD _asbp_main_character)) "Hidden"))

(event EventBeginPlay)

(event Collision|EventActorBeginOverlap
  (params (OtherActor :type Actor%20Object%20Reference)))

(event EventTick
  (params (DeltaSeconds :type Float%20%28single-precision%29))
  (bind _eventlistener (Variables|Default|GetEventListener))
  (if (not (and (Class|EventListenerComponent|IsIsinAEventTask _eventlistener) (not (Class|EventListenerComponent|IsIsActorEnable _eventlistener))))
    (if (not (Variables|Default|GetIsActivated))
      (Variables|Default|SetIsActivated true)
      (Class|EventListenerComponent|TaskCompleted (Variables|Default|GetEventListener) self)
      (CallFunction|ExecSound1)
      (Utilities|FlowControl|Delay 6.0)
      (CallFunction|ExecSound2)
      (Utilities|FlowControl|Delay 4.0)
      (CallFunction|ExecSound3)
      (Utilities|FlowControl|Delay 4.0)
      (CallFunction|ExecSound4)
      (Utilities|FlowControl|Delay 4.0)
      (CallFunction|ExecSound5))))

(fn ConstructionScript)