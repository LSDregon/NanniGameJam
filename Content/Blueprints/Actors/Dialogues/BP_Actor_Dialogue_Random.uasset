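; Dialogue actor that plays a one-time voice line with on-screen text for the main character.
; On Tick, once its EventListener allows it (not in an event task, or enabled), it latches and reports the task completed.
; It shows the text on the HUD's spring overlay with 2D audio, hiding it after a fixed delay.
; Despite the name, it always reads AudioText key 0; the random-index node is unused.
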(event EventBeginPlay)

(event Collision|EventActorBeginOverlap
  (params (OtherActor :type Actor%20Object%20Reference)))

(event EventTick
  (params (DeltaSeconds :type Float%20%28single-precision%29))
  (bind _eventlistener (Variables|Default|GetEventListener))
  (if (not (and (Class|EventListenerComponent|IsIsinAEventTask _eventlistener) (not (Class|EventListenerComponent|IsIsActorEnable _eventlistener))))
    (if (not (Variables|Default|GetIsActivated))
      (Variables|Default|SetIsActivated true)
      (Class|EventListenerComponent|TaskCompleted (Variables|Default|GetEventListener) self)
      (bind (_bstruct _text _sound) (CallFunction|GetRandomStruct))
      (bind _asbp_main_character (Utilities|Casting|CastToBP_MainCharacter (Game|GetPlayerCharacter 0)))
      (Default|SetTextSpring (Variables|/Game/Blueprints/MainPlayer/BP_MainCharacter.BP_MainCharacter_C|GetHUD _asbp_main_character) _text)
      (Widget|SetVisibility (Variables|/Game/Blueprints/MainPlayer/WBP_HUD.WBP_HUD_C|GetOverlay_Spring (Variables|/Game/Blueprints/MainPlayer/BP_MainCharacter.BP_MainCharacter_C|GetHUD _asbp_main_character)) "Visible")
      (Audio|PlaySound2D _sound 1.0 1.0 0.0 0 0)
      (Utilities|FlowControl|Delay 7.0)
      (Widget|SetVisibility (Variables|/Game/Blueprints/MainPlayer/WBP_HUD.WBP_HUD_C|GetOverlay_Spring (Variables|/Game/Blueprints/MainPlayer/BP_MainCharacter.BP_MainCharacter_C|GetHUD _asbp_main_character)) "Hidden"))))

(fn ConstructionScript)

(fn GetRandomStruct
  (bind _audio_text (Variables|Default|GetAudio_Text))
  (bind (_value _returnvalue) (Utilities|Map|Find _audio_text 0))
  (bind (_sound _text) (Utilities|Struct|BreakStruct_Audio_Text _value))
  (return _returnvalue _text _sound))