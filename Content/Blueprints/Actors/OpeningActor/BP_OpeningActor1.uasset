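; BP_OpeningActor1 is an interactable actor that shows a random voice or text line to the player.
; On interaction it plays a door/window sound at its location and gets a random text and audio pair from the AudioText map via GetRandomStruct.
; It displays the text in the main character's HUD spring overlay, plays the audio in 2D, then hides the overlay after a fixed delay.
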(event OnInteract(InteractionComponent)
  (params (Character :type Main%20Character%20Object%20Reference))
  (Audio|PlaySoundatLocation "/Game/Sounds/SoundsWaves/Props/MS_Door_Windows.MS_Door_Windows" (Transformation|GetActorLocation) "0, 0, 0" 1.0 1.0 0.0 0 0 0 0)
  (bind (_bstruct _text _sound) (CallFunction|GetRandomStruct))
  (bind _asbp_main_character (Utilities|Casting|CastToBP_MainCharacter (Game|GetPlayerCharacter 0)))
  (Default|SetTextSpring (Variables|/Game/Blueprints/MainPlayer/BP_MainCharacter.BP_MainCharacter_C|GetHUD _asbp_main_character) _text)
  (Widget|SetVisibility (Variables|/Game/Blueprints/MainPlayer/WBP_HUD.WBP_HUD_C|GetOverlay_Spring (Variables|/Game/Blueprints/MainPlayer/BP_MainCharacter.BP_MainCharacter_C|GetHUD _asbp_main_character)) "Visible")
  (Audio|PlaySound2D _sound 1.0 1.0 0.0 0 0)
  (Utilities|FlowControl|Delay 1e+01)
  (Widget|SetVisibility (Variables|/Game/Blueprints/MainPlayer/WBP_HUD.WBP_HUD_C|GetOverlay_Spring (Variables|/Game/Blueprints/MainPlayer/BP_MainCharacter.BP_MainCharacter_C|GetHUD _asbp_main_character)) "Hidden"))

(fn ConstructionScript)

(fn GetRandomStruct
  (bind _audio_text (Variables|Default|GetAudio_Text))
  (bind _audio_text_2 (Variables|Default|GetAudio_Text))
  (bind _returnvalue (Utilities|Map|Length _audio_text_2))
  (bind _returnvalue_2 (Math|Random|RandomIntegerinRange 1 _returnvalue))
  (bind (_value _returnvalue_3) (Utilities|Map|Find _audio_text _returnvalue_2))
  (bind (_text _audio) (Utilities|Struct|BreakStruct_Audio_Text_Dialogue _value))
  (return _returnvalue_3 _text _audio))