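; BP_Teleport is a single-use-per-activation portal that teleports the player character.
; It starts with both portal effects off until the ActivatePortal event arms it and turns them on.
; When the player enters the Box while it is active, they move to the Arrow component's location and rotation.
; The portal then disarms immediately and switches both effects off after a short delay.
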(event OnComponentBeginOverlap(Box)
  (params (OverlappedComponent :type Primitive%20Component%20Object%20Reference) (OtherActor :type Actor%20Object%20Reference) (OtherComp :type Primitive%20Component%20Object%20Reference) (OtherBodyIndex :type Integer) (bFromSweep :type Boolean) (SweepResult :type Hit%20Result%20Structure%20%28by%20ref%29))
  (bind _returnvalue (Game|GetPlayerCharacter 0))
  (bind _arrow (Variables|Default|GetArrow))
  (if (== OtherActor _returnvalue)
    (if (Variables|Default|GetIsActive)
      (Transformation|SetActorLocationAndRotation _returnvalue (Transformation|GetWorldLocation _arrow) (Transformation|GetWorldRotation _arrow) false true)
      (Variables|Default|SetIsActive false)
      (Utilities|FlowControl|Delay 1.0)
      (Components|Activation|Deactivate (Variables|Default|GetVFXPortal))
      (Components|Activation|Deactivate (Variables|Default|GetVFXPortal1)))))

(event Custom|ActivatePortal
  (Variables|Default|SetIsActive true)
  (Components|Activation|Activate (Variables|Default|GetVFXPortal) false)
  (Components|Activation|Activate (Variables|Default|GetVFXPortal1) false))

(event EventBeginPlay
  (Components|Activation|Deactivate (Variables|Default|GetVFXPortal))
  (Components|Activation|Deactivate (Variables|Default|GetVFXPortal1)))

(fn ConstructionScript)