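; Behavior tree task that switches the Nanni enemy's pawn collision according to an activation flag.
; It casts and caches the Nanni character and controller, then sets the root capsule to block and the secondary capsule to overlap pawns, or both to ignore when inactive.
; Both branches make the capsule hierarchy visible, and the AI perception toggles are disconnected.
; The task never calls Finish Execute.
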(event EventReceiveExecuteAI
  (params (OwnerController :type AI%20Controller%20Object%20Reference) (ControlledPawn :type Pawn%20Object%20Reference))
  (bind _asbp_enemy_nanni_character (Utilities|Casting|CastToBP_EnemyNanniCharacter ControlledPawn))
  (Variables|Default|SetAs%20BP%20Enemy%20Nanni%20Character _asbp_enemy_nanni_character)
  (bind _asbp_enemy_nanni_controller (Utilities|Casting|CastToBP_EnemyNanniController OwnerController))
  (Variables|Default|SetAs%20BP%20Enemy%20Nanni%20Controller _asbp_enemy_nanni_controller)
  (if (Variables|Default|GetIsActivationProcess)
    (Rendering|SetVisibility (Variables|/Script/Engine.Character|GetCapsuleComponent (Variables|Default|GetAs%20BP%20Enemy%20Nanni%20Character)) true true)
    (Collision|SetCollisionResponsetoChannel (Variables|/Script/Engine.Character|GetCapsuleComponent (Variables|Default|GetAs%20BP%20Enemy%20Nanni%20Character)) "ECC_Pawn" "ECR_Block")
    (Collision|SetCollisionResponsetoChannel (Variables|/Game/Blueprints/Enemy/Nanni/BP_EnemyNanniCharacter.BP_EnemyNanniCharacter_C|GetCapsule (Variables|Default|GetAs%20BP%20Enemy%20Nanni%20Character)) "ECC_Pawn" "ECR_Overlap")
    (else
      (Rendering|SetVisibility (Variables|/Script/Engine.Character|GetCapsuleComponent (Variables|Default|GetAs%20BP%20Enemy%20Nanni%20Character)) true true)
      (Collision|SetCollisionResponsetoChannel (Variables|/Script/Engine.Character|GetCapsuleComponent (Variables|Default|GetAs%20BP%20Enemy%20Nanni%20Character)) "ECC_Pawn" "ECR_Ignore")
      (Collision|SetCollisionResponsetoChannel (Variables|/Game/Blueprints/Enemy/Nanni/BP_EnemyNanniCharacter.BP_EnemyNanniCharacter_C|GetCapsule (Variables|Default|GetAs%20BP%20Enemy%20Nanni%20Character)) "ECC_Pawn" "ECR_Ignore"))))